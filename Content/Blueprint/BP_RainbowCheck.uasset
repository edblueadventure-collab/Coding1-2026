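; BP_RainbowCheck is a checkpoint actor that saves a respawn-style position on the player's BP_ThirdPersonCharacter.
; Overlapping its Box writes the Box's world location to the character's LastSavedPosition and prints a confirmation.
; A separate actor overlap creates a dynamic material on the Flag and sets a random RandomColor entry as a vector parameter, though the parameter name is left as None.
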(event OnComponentBeginOverlap(Box)
  (params (OverlappedComponent :type Primitive%20Component%20Object%20Reference) (OtherActor :type Actor%20Object%20Reference) (OtherComp :type Primitive%20Component%20Object%20Reference) (OtherBodyIndex :type Integer) (bFromSweep :type Boolean) (SweepResult :type Hit%20Result%20Structure%20%28by%20ref%29))
  (bind _asbp_third_person_character (Utilities|Casting|CastToBP_ThirdPersonCharacter OtherActor))
  (Variables|/Game/ThirdPerson/Blueprints/BP_ThirdPersonCharacter.BP_ThirdPersonCharacter_C|SetLastSavedPosition _asbp_third_person_character (Transformation|GetWorldLocation (Variables|Default|GetBox)))
  (Development|PrintText "Check Point Found!"))

(event EventBeginPlay)

(event Collision|EventActorBeginOverlap
  (params (OtherActor :type Actor%20Object%20Reference))
  (Utilities|Casting|CastToBP_ThirdPersonCharacter OtherActor)
  (bind _returnvalue (Rendering|Material|CreateDynamicMaterialInstance (Variables|Default|GetFlag) 0 0 "None" :!class /Script/Engine.PrimitiveComponent))
  (Variables|Default|SetDynamic%20Color _returnvalue)
  (Rendering|Material|SetVectorParameterValue 0 "None" (.OutItem (Utilities|Array|Random (Variables|Default|GetRandomColor))) :!class /Script/Engine.KismetMaterialLibrary))

(event EventTick
  (params (DeltaSeconds :type Float%20%28single-precision%29)))

(fn ConstructionScript)