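; BP_DialogueManager is a dialogue manager that shows lines from a Dialogue array as debug printed text.
; Its Displaynextline event checks Index against the array length, prints the entry at Index, then increments it.
; The check resets Index to zero while it is still below the length, so valid calls repeat the first line instead of advancing.
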(event Custom|Display%20next%20line
  (if (>= (Variables|Default|Getindex) (Utilities|Array|Length (Variables|Default|GetDialogue)))
    _
    (else
      (Variables|Default|Setindex 0)))
  (Development|PrintText (Utilities|Array|Get(acopy) (Variables|Default|GetDialogue) (Variables|Default|Getindex)))
  (Math|Integer|IncrementInt (Variables|Default|Getindex)))

(event EventBeginPlay)

(event Collision|EventActorBeginOverlap
  (params (OtherActor :type Actor%20Object%20Reference)))

(event EventTick
  (params (DeltaSeconds :type Float%20%28single-precision%29)))

(fn ConstructionScript)