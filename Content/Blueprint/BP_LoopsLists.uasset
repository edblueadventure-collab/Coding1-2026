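; BP_LoopsLists is a demo Blueprint of loops and arrays that prints debug text and moves the level's keys.
; BeginPlay uses a Sequence with two delayed branches: a While loop printing a countdown in colors cycled by modulo, and a call to Makecoinsjump.
; Makecoinsjump gathers every BP_Key, nudges each root component upward, prints the count, then calls itself after a Delay, so keys keep rising indefinitely.
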(event Custom|makecoinsjump
  (bind _outactors (Actor|GetAllActorsOfClass "/Game/Blueprint/BP_Key.BP_Key_C"))
  (for _array_element _outactors
    (Transformation|AddRelativeLocation (Variables|/Game/Blueprint/BP_Key.BP_Key_C|GetDefaultSceneRoot _array_element) "0.000000,0.000000,50.000000" false false))
  (Development|PrintText (Utilities|Text|FormatText "We have raised {count} keys" (Utilities|Array|Length _outactors)))
  (Utilities|FlowControl|Delay 1.0)
  (CallFunction|Makecoinsjump) ; Function call itself one second after completion
)

(event EventBeginPlay
  (bind _whilecounter (Variables|Default|GetWhilecounter))
  (Utilities|FlowControl|Sequence
    (:then_0
      (Utilities|FlowControl|Delay 0.2)
      (while (> _whilecounter 0)
        (Development|PrintText (Utilities|Text|FormatText "We are in Loop number{Count}" _whilecounter) true true (Utilities|Array|Get(acopy) (Variables|Default|GetColors) (Math|Integer|%(Integer) (Variables|Default|GetWhilecounter) 7)) 22.0)
        (Math|Integer|DecrementInt (Variables|Default|GetWhilecounter))))
    (:then_1
      (Utilities|FlowControl|Delay 1.0)
      (CallFunction|Makecoinsjump))))

(event Collision|EventActorBeginOverlap
  (params (OtherActor :type Actor%20Object%20Reference)))

(event EventTick
  (params (DeltaSeconds :type Float%20%28single-precision%29)))

(fn ConstructionScript)