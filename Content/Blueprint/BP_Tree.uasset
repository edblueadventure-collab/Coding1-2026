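; Tree actor Blueprint that grows its static mesh in stages after play begins.
; On BeginPlay it loops while GrowCount is above zero: it waits a random few seconds, adds a random increment to the mesh's relative scale, then decrements the count.
; An unconnected leftover chain that sets random scales after short delays never runs, and the construction script is empty.
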(event EventBeginPlay
  (bind _staticmesh (Variables|Default|GetStaticMesh))
  (if (> (Variables|Default|GetGrowCount) 0) :!label _label
    (Utilities|FlowControl|Delay (Math|Random|RandomFloatinRange 4.0 6.0))
    (Transformation|SetRelativeScale3D _staticmesh (+ (Variables|/Script/Engine.SceneComponent|GetRelativeScale3D _staticmesh) (Math|Random|RandomFloatinRange 0.4 0.6)))
    (Math|Integer|DecrementInt (Variables|Default|GetGrowCount)
      (:%20%20
        (goto _label)))))

(event Collision|EventActorBeginOverlap
  (params (OtherActor :type Actor%20Object%20Reference)))

(event EventTick
  (params (DeltaSeconds :type Float%20%28single-precision%29)))

(fn ConstructionScript)