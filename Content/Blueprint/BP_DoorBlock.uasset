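; BP_DoorBlock is a locked door that opens once enough keys have been collected.
; Each CollectItem call increments the key count, and on reaching the maximum a DoOnce fires OpenDoor and destroys the Lock component.
; OpenDoor plays a Timeline that swings the door mesh open by lerping its relative yaw and disables its collision during the animation.
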(event Custom|Open%20Door
  (bind _newtrack_0 (Timeline|Timeline Play)
    (:Update
      (Transformation|SetRelativeRotation (Variables|Default|GetSM_Bld_Door_01) (Math|Rotator|Lerp(Rotator) "0, 0, 0" "0.000000,-110.000000,0.000000" _newtrack_0) false false)
      (Collision|SetCollisionEnabled (Variables|Default|GetSM_Bld_Door_01) "NoCollision"))))

(event Custom|CollectItem
  (Math|Integer|IncrementInt (Variables|Default|GetCurrentKeysCollected)
    (:%20%20
      (if (>= (Variables|Default|GetCurrentKeysCollected) (Variables|Default|GetMaxKeysCollected))
        (Utilities|FlowControl|DoOnce false
          (:Completed
            (CallFunction|OpenDoor)
            (Components|DestroyComponent (Variables|Default|Getlock))))))))

(event EventBeginPlay)

(event Collision|EventActorBeginOverlap
  (params (OtherActor :type Actor%20Object%20Reference)))

(event EventTick
  (params (DeltaSeconds :type Float%20%28single-precision%29)))

(fn ConstructionScript)