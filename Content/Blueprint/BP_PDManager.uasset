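; BP_PDManager is a dialogue manager that shows lines from a Dialogue array one at a time.
; It creates a UI_RickRoll widget at BeginPlay and reuses it for every line.
; Each Displaythenextline call prints the current line, calls ShowUI and advances Index, doing nothing once the array is exhausted.
; ShowUI sets the widget's text, adds it to the viewport and removes it after a short delay.
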(event Custom|Display%20the%20next%20line
  (if (not (>= (Variables|Default|Getindex) (Utilities|Array|Length (Variables|Default|GetDialogue))))
    (Development|PrintText (Utilities|Array|Get(acopy) (Variables|Default|GetDialogue) (Variables|Default|Getindex)) true true "(R=0.000000,G=0.660000,B=1.000000,A=1.000000)" 5.0)
    (CallFunction|ShowUI)
    (Math|Integer|IncrementInt (Variables|Default|Getindex))))

(event Custom|ShowUI
  (bind _widget (Variables|Default|GetWidget))
  (Rendering|Components|TextRender|SetText (Variables|/Game/Widgets/UI_RickRoll.UI_RickRoll_C|GetTextBlock_2 (Variables|Default|GetWidget)) (Utilities|Array|Get(acopy) (Variables|Default|GetDialogue) (Variables|Default|Getindex)))
  (UserInterface|Viewport|AddtoViewport _widget 0)
  (Utilities|FlowControl|Delay 3.5)
  (Widget|RemovefromParent _widget))

(event EventBeginPlay
  (bind _returnvalue (UserInterface|CreateWidget "/Game/Widgets/UI_RickRoll.UI_RickRoll_C"))
  (Variables|Default|SetWidget _returnvalue))

(event Collision|EventActorBeginOverlap
  (params (OtherActor :type Actor%20Object%20Reference)))

(event EventTick
  (params (DeltaSeconds :type Float%20%28single-precision%29)))

(fn ConstructionScript)