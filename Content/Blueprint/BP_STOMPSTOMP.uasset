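; BP_STOMPSTOMP is a stomping spike trap that drops when the player passes beneath it.
; Each Tick it traces downward, and a BP_ThirdPersonCharacter hit plays the Stompage timeline, lerping Spikeblock's relative location downward from its current value.
; Overlapping the Box teleports the character to its LastSavedPosition.
; The HasChecked branch has a constant false condition, so that flag is never set.
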(event OnComponentBeginOverlap(Box)
  (params (OverlappedComponent :type Primitive%20Component%20Object%20Reference) (OtherActor :type Actor%20Object%20Reference) (OtherComp :type Primitive%20Component%20Object%20Reference) (OtherBodyIndex :type Integer) (bFromSweep :type Boolean) (SweepResult :type Hit%20Result%20Structure%20%28by%20ref%29))
  (bind _asbp_third_person_character (Utilities|Casting|CastToBP_ThirdPersonCharacter OtherActor))
  (Transformation|SetActorLocation _asbp_third_person_character (Variables|/Game/ThirdPerson/Blueprints/BP_ThirdPersonCharacter.BP_ThirdPersonCharacter_C|GetLastSavedPosition _asbp_third_person_character) false false))

(event EventBeginPlay)

(event Collision|EventActorBeginOverlap
  (params (OtherActor :type Actor%20Object%20Reference)))

(event EventTick
  (params (DeltaSeconds :type Float%20%28single-precision%29))
  (bind _returnvalue (Transformation|GetActorLocation))
  (bind _outhit (Collision|LineTraceByChannel _returnvalue (+ _returnvalue "0.000000,0.000000,-1000.000000") "TraceTypeQuery1" false 0 "ForDuration"))
  (Utilities|Casting|CastToBP_ThirdPersonCharacter (.HitActor (Collision|BreakHitResult _outhit)))
  (if false
    (Variables|Default|SetHasChecked true)
    (else
      (bind _newtrack_0 (Timeline|Stompage Play)
        (:Update
          (Transformation|SetRelativeLocation (Variables|Default|Getspike-block) (Math|Vector|Lerp(Vector) (Variables|/Script/Engine.SceneComponent|GetRelativeLocation (Variables|Default|Getspike-block)) "0.000000,0.000000,-1000.000000" _newtrack_0) false false))))))

(fn ConstructionScript)