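; BP_FRainbowCheckpoint is a checkpoint actor with a flag that responds when a BP_ThirdPersonCharacter overlaps it.
; Overlapping the Box saves its world location as the character's LastSavedPosition.
; A separate actor-level overlap creates a dynamic material on the Flag and sets a vector parameter to a random Color entry, though the parameter name is None.
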(event OnComponentBeginOverlap(Box)
  (params (OverlappedComponent :type Primitive%20Component%20Object%20Reference) (OtherActor :type Actor%20Object%20Reference) (OtherComp :type Primitive%20Component%20Object%20Reference) (OtherBodyIndex :type Integer) (bFromSweep :type Boolean) (SweepResult :type Hit%20Result%20Structure%20%28by%20ref%29))
  (bind _asbp_third_person_character (Utilities|Casting|CastToBP_ThirdPersonCharacter OtherActor))
  (Variables|/Game/ThirdPerson/Blueprints/BP_ThirdPersonCharacter.BP_ThirdPersonCharacter_C|SetLastSavedPosition _asbp_third_person_character (Transformation|GetWorldLocation (Variables|Default|GetBox))))

(event EventBeginPlay)

(event Collision|EventActorBeginOverlap
  (params (OtherActor :type Actor%20Object%20Reference))
  (Utilities|Casting|CastToBP_ThirdPersonCharacter OtherActor)
  (bind _returnvalue (Rendering|Material|CreateDynamicMaterialInstance (Variables|Default|Getflag) 0 0 "None" :!class /Script/Engine.PrimitiveComponent))
  (Variables|Default|SetMAT _returnvalue)
  (Rendering|Material|SetVectorParameterValue 0 "None" (.OutItem (Utilities|Array|Random (Variables|Default|GetColor))) :!class /Script/Engine.KismetMaterialLibrary))

(fn ConstructionScript)